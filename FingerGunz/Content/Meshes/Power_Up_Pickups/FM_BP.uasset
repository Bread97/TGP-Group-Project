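; FM_BP is a pickup actor with a FiringBoost component that spins and temporarily disappears when overlapped.
; Tick rotates FiringBoost around its yaw axis at a constant, frame-rate-independent speed.
; Any actor overlap hides the component and disables collision, then a short delay restores both so the pickup respawns in place.
; The graph itself applies no boost effect to the overlapping actor.
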(event `self.ReceiveTick`
  (params (DeltaSeconds :type "Float (single-precision)"))
  (`SceneComponent.K2_AddLocalRotation` (`self.firing_boost`) (`KismetMathLibrary.MakeRotator` 0.0 0.0 (* DeltaSeconds 90.0)) false false))

(event `self.ReceiveActorBeginOverlap`
  (params (OtherActor :type "Actor Object Reference"))
  (`SceneComponent.SetVisibility` (`self.firing_boost`) false false)
  (`self.SetActorEnableCollision` false)
  (`KismetSystemLibrary.Delay` 5.0)
  (`SceneComponent.SetVisibility` (`self.firing_boost`) true false)
  (`self.SetActorEnableCollision` true))

(fn `UserConstructionScript`)