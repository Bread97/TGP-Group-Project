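; Shield power-up pickup that rotates in place and sets the player's Armour to 50 when it differs from MaxShield.
; Beginning overlap plays two staggered sounds, then hides the shield and disables actor collision for five seconds before it respawns.
; The Armour change itself happens in the end-overlap event, which repeats the MaxShield check.
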(event `self.ReceiveTick`
  (params (DeltaSeconds :type "Float (single-precision)"))
  (`SceneComponent.K2_AddLocalRotation` (`self.shield`) (`KismetMathLibrary.MakeRotator` 0.0 0.0 (* DeltaSeconds 90.0)) false false))

(event `self.ReceiveActorBeginOverlap`
  (params (OtherActor :type "Actor Object Reference"))
  (bind _asplayer_blue_print (cast `/Game/Player/Player_BluePrint` OtherActor))
  ;[1 1 1] If the player's shields are at max, do not allow interaction
  (if (!= (`/Game/Player/Player_BluePrint.Armour` _asplayer_blue_print) (`self.MaxShield`))
    (`|ExecutionSequence`
      (:`then_0`
        (`SceneComponent.SetVisibility` (`self.shield`) false false)
        (`self.SetActorEnableCollision` false)
        (`KismetSystemLibrary.Delay` 5.0)
        (`SceneComponent.SetVisibility` (`self.shield`) true false)
        (`self.SetActorEnableCollision` true))
      (:`then_1`
        (`GameplayStatics.PlaySound2D` "/Game/Audio/SFX/PowerUp_Pickups/Shield_Pickup_Cue.Shield_Pickup_Cue" 1.0 1.0 0.0 null null)
        (`KismetSystemLibrary.Delay` 0.2)
        (`GameplayStatics.PlaySound2D` "/Game/Audio/SFX/PowerUp_Pickups/Shield_Pickup_Effect_Cue.Shield_Pickup_Effect_Cue" 1.0 1.0 0.0 null null)))))

(event `self.ReceiveActorEndOverlap`
  (params (OtherActor :type "Actor Object Reference"))
  (bind _asplayer_blue_print (cast `/Game/Player/Player_BluePrint` OtherActor))
  ;[1 1 1] If the player is at full health, do not allow Healing
  (if (!= (`/Game/Player/Player_BluePrint.Armour` _asplayer_blue_print) (`self.MaxShield`))
    (set `/Game/Player/Player_BluePrint.Armour` 50 _asplayer_blue_print)))

(fn `UserConstructionScript`)