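; Speed boost pickup whose SpeedUp component spins steadily around yaw.
; On begin overlap, it hides and disables collision, then reappears with collision restored after a delay.
; On end overlap, a timeline restarts and drives the overlapping Character's MaxWalkSpeed from its SpeedUpTrack curve.
; Begin overlap does not filter by actor type, and the RespawnShield function is empty.
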(event `self.ReceiveTick`
  (params (DeltaSeconds :type "Float (single-precision)"))
  (`SceneComponent.K2_AddLocalRotation` (`self.speed_up`) (`KismetMathLibrary.MakeRotator` 0.0 0.0 (* DeltaSeconds 90.0)) false false))

(event `self.ReceiveActorEndOverlap`
  (params (OtherActor :type "Actor Object Reference"))
  (bind _ascharacter (cast `Character` OtherActor))
  (bind (_direction _speeduptrack) (`Timeline|Spd_Up_Timeline` :!via `PlayFromStart`)
    (:`Update`
      (set `CharacterMovementComponent.MaxWalkSpeed` _speeduptrack (`Character.CharacterMovement` _ascharacter)))))

(event `self.ReceiveActorBeginOverlap`
  (params (OtherActor :type "Actor Object Reference"))
  (`SceneComponent.SetVisibility` (`self.speed_up`) false false)
  (`self.SetActorEnableCollision` false)
  (`KismetSystemLibrary.Delay` 5.0)
  (`SceneComponent.SetVisibility` (`self.speed_up`) true false)
  (`self.SetActorEnableCollision` true))

(fn `RespawnShield`)

(fn `UserConstructionScript`)