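; Health pickup Blueprint that spins its Heal mesh and restores HP to a Player_BluePrint that is not at MaxHP.
; Begin overlap plays Heal_Cue, hides the mesh and disables collision, then restores both after a short delay so the pickup respawns.
; End overlap adds HealVal to the player's HP, with no clamp to MaxHP.
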(event `self.ReceiveTick`
  (params (DeltaSeconds :type "Float (single-precision)"))
  (`SceneComponent.K2_AddLocalRotation` (`self.heal`) (`KismetMathLibrary.MakeRotator` 0.0 0.0 (* DeltaSeconds 90.0)) false false))

(event `self.ReceiveActorBeginOverlap`
  (params (OtherActor :type "Actor Object Reference"))
  (bind _asplayer_blue_print (cast `/Game/Player/Player_BluePrint` OtherActor))
  ;[1 1 1] If the player is at full health, do not allow interaction
  (if (!= (`/Game/Player/Player_BluePrint.HP` _asplayer_blue_print) (`self.MaxHP`))
    (`|ExecutionSequence`
      (:`then_0`
        (`SceneComponent.SetVisibility` (`self.heal`) false false)
        (`self.SetActorEnableCollision` false)
        (`KismetSystemLibrary.Delay` 5.0)
        (`SceneComponent.SetVisibility` (`self.heal`) true false)
        (`self.SetActorEnableCollision` true))
      (:`then_1`
        (`GameplayStatics.PlaySound2D` "/Game/Audio/SFX/PowerUp_Pickups/Heal_Cue.Heal_Cue" 1.0 1.0 0.0 null null)))))

(event `self.ReceiveActorEndOverlap`
  (params (OtherActor :type "Actor Object Reference"))
  (bind _asplayer_blue_print (cast `/Game/Player/Player_BluePrint` OtherActor))
  ;[1 1 1] If the player is at full health, do not allow Healing
  (if (!= (`/Game/Player/Player_BluePrint.HP` _asplayer_blue_print) (`self.MaxHP`))
    ;[1 1 1] Apply Healing to Player
    (set `/Game/Player/Player_BluePrint.HP` (+ (`/Game/Player/Player_BluePrint.HP` _asplayer_blue_print) (`self.HealVal`)) _asplayer_blue_print)))

(fn `UserConstructionScript`)