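; Shotgun weapon pickup actor that spins in place and respawns 30 seconds after being touched.
; Begin overlap from any actor hides the mesh and disables collision, restoring both after the delay.
; The grant happens on end overlap: if the actor is the player Blueprint, it sets the shotgun picked-up flag and plays two staggered pickup sounds.
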(event `self.ReceiveTick`
  (params (DeltaSeconds :type "Float (single-precision)"))
  (`SceneComponent.K2_AddLocalRotation` (`self.shotgun_pickup`) (`KismetMathLibrary.MakeRotator` 0.0 (* DeltaSeconds 90.0)) false false))

(event `self.ReceiveActorBeginOverlap`
  (params (OtherActor :type "Actor Object Reference"))
  (`SceneComponent.SetVisibility` (`self.shotgun_pickup`) false false)
  (`self.SetActorEnableCollision` false)
  (`KismetSystemLibrary.Delay` 30.0)
  (`SceneComponent.SetVisibility` (`self.shotgun_pickup`) true false)
  (`self.SetActorEnableCollision` true))

(event `self.ReceiveActorEndOverlap`
  (params (OtherActor :type "Actor Object Reference"))
  (bind _asplayer_blue_print (cast `/Game/Player/Player_BluePrint` OtherActor))
  (set `/Game/Player/Player_BluePrint.Shotgun_Picked_Up` true _asplayer_blue_print)
  (`GameplayStatics.PlaySound2D` "/Game/Audio/SFX/Shotgun_SFX/Shotgun_Pickup_Pump_SFX_Cue.Shotgun_Pickup_Pump_SFX_Cue" 1.0 1.0 0.0 null null)
  (`KismetSystemLibrary.Delay` 0.2)
  (`GameplayStatics.PlaySound2D` "/Game/Audio/SFX/Shotgun_SFX/Shotgun_Pickup_SFX_Cue.Shotgun_Pickup_SFX_Cue" 1.0 1.0 0.0 null null))

(fn `UserConstructionScript`)